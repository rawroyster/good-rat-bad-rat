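; BP_Dummy is a melee enemy character that chases the player on sight and punches them.
; PawnSensing sets a seen flag and starts an AIMoveTo toward the player, then a punch montage gated by CanAttack for its duration.
; Tick halts movement until the player is seen, and the flag effectively stays set afterward.
; AnyDamage reduces Health, destroying the actor on a hit received at zero or below.
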(event OnSeePawn(PawnSensing)
  (params (Pawn :type Pawn%20Object%20Reference))
  (Variables|Default|SetIsSeeingPlayer true)
  (CallFunction|FollowPlayer))

(event Custom|FollowPlayer
  (Variables|Default|SetCanAttack true)
  (if (Variables|Default|GetIsSeeingPlayer)
    (AI|AIMoveTo self "0, 0, 0" (Game|GetPlayerCharacter 0) 7e+01 false
      (:OnSuccess
        (if (Variables|Default|GetCanAttack)
          (Variables|Default|SetCanAttack false)
          (bind _returnvalue (Animation|PlayAnimMontage "/Game/Characters/Animations/AI/H2H_PunchCombo03_Montage.H2H_PunchCombo03_Montage" 1.0 "None"))
          (Utilities|FlowControl|Delay _returnvalue)
          (Variables|Default|SetCanAttack true))))
    (else
      (Variables|Default|SetIsSeeingPlayer false))))

(event EventBeginPlay)

(event Collision|EventActorBeginOverlap
  (params (OtherActor :type Actor%20Object%20Reference)))

(event EventTick
  (params (DeltaSeconds :type Float%20%28single-precision%29))
  (if (not (Variables|Default|GetIsSeeingPlayer))
    (Components|Movement|StopMovementImmediately (Variables|Character|GetCharacterMovement))))

(event Game|Damage|EventAnyDamage
  (params (Damage :type Float%20%28single-precision%29) (DamageType :type Damage%20Type%20Object%20Reference) (InstigatedBy :type Controller%20Object%20Reference) (DamageCauser :type Actor%20Object%20Reference))
  (if (> (Variables|Default|GetHealth) 0.0)
    (Variables|Default|SetHealth (- (Variables|Default|GetHealth) Damage))
    (Development|PrintString "Damage received")
    (else
      (Actor|DestroyActor))))

(fn ConstructionScript)